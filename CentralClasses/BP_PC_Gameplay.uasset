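; Gameplay player controller that runs the UI and input for Elestral team management and clashes, plus pause, settings, dialogue and the compendium.
; Input toggles open the time-slowed clash swap menu, a team display that eases into pause, or a possessed compendium actor.
; Team, summary (3D preview) and skill tree screens edit the character team component's stat list, syncing move changes to the following Elestral.
; Clash events manage the clash HUD and its health and bond meters.
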(event `SendOutSwappedElestralInClash`
  (params (StatsToInitWith :type "ElestralStats Structure"))
  (bind _player_elestral_team_component (`self.Player Elestral Team Component`))
  (`AC_ElestralsTeamComponent.SwapElestralTeamPositions` _player_elestral_team_component (`KismetArrayLibrary.Array_Find` (`AC_ElestralsTeamComponent.TeamStatList` _player_elestral_team_component) StatsToInitWith) 0)
  (`self.DestroySwapWidget`)
  (message `/Game/Blueprints/CentralClasses/BPI_ClashUtils.NotifyGameStateElestralWasSwapped` (`GameplayStatics.GetGameState`) true (cast `/Game/Blueprints/Elestrals/BP_ElestralBase` (`AC_ElestralsTeamComponent.CurrentFollowingElestral` (`self.Player Elestral Team Component`)) :!pure true)))

(event `/Game/Blueprints/CentralClasses/BPI_UIUtils.UpdateNexusedElestralInController`
  (params (Index :type Integer) (StatStruct :type "ElestralStats Structure"))
  (`self.NexusPlayerElestral` Index StatStruct))

(event `EnhancedInput|/Game/ThirdPerson/Input/Actions/IA_SwapAction`
  (params (ActionValue :type Boolean) (ElapsedSeconds :type "Float (double-precision)") (TriggeredSeconds :type "Float (double-precision)") (InputAction :type "InputAction Object Reference" :default "/Game/ThirdPerson/Input/Actions/IA_SwapAction.IA_SwapAction"))
  (:`Started`
    (if (`self.isInClash`) :!label _label
      (`/Engine/EditorBlueprintResources/StandardMacros.FlipFlop`
        (:`A`
          (bind _returnvalue (`|CreateWidget` "/Game/UserInterface/Clash/WB_ClashSwap.WB_ClashSwap_C" null self))
          (bind _output_get (set `self.ClashSwapWidgetRef` _returnvalue))
          (`UserWidget.AddToViewport` _output_get 0)
          (set `self.bShowMouseCursor` true)
          (`/Game/UserInterface/Clash/WB_ClashSwap.InitializeSwapButtons` (`self.ClashSwapWidgetRef`) (`AC_ElestralsTeamComponent.TeamStatList` (`self.Player Elestral Team Component`)))
          (`GameplayStatics.SetGlobalTimeDilation` 0.1))
        (:`B`
          (`Widget.RemoveFromParent` (`self.ClashSwapWidgetRef`))
          (set `self.bShowMouseCursor` false)
          (`GameplayStatics.SetGlobalTimeDilation` 1.0)
          (`WidgetBlueprintLibrary.SetInputMode_GameOnly` self))))))

(event `DestroySwapWidget`
  (goto _label))

(event `EnhancedInput|/Game/ThirdPerson/Input/Actions/IA_DisplayTeam`
  (params (ActionValue :type Boolean) (ElapsedSeconds :type "Float (double-precision)") (TriggeredSeconds :type "Float (double-precision)") (InputAction :type "InputAction Object Reference" :default "/Game/ThirdPerson/Input/Actions/IA_DisplayTeam.IA_DisplayTeam"))
  (bind _elestralsteamdisplayref (`self.ElestralsTeamDisplayRef`))
  ;[1 1 1] TeamDisplay Widget Appear and Initialize Logic
  (:`Started`
    (if (not (`self.isInputtingCombo`))
      (`/Engine/EditorBlueprintResources/StandardMacros.FlipFlop`
        (:`A`
          (if (not (`self.isInClash`))
            (bind _returnvalue (`|CreateWidget` "/Game/UserInterface/Widgets/WB_TeamDisplay.WB_TeamDisplay_C"))
            (bind _output_get (set `self.ElestralsTeamDisplayRef` _returnvalue))
            (`UserWidget.AddToViewport` _output_get 0)
            (for (_array_element _array_index) (`AC_ElestralsTeamComponent.TeamStatList` (`self.Player Elestral Team Component`))
              (bind _returnvalue_2 (`|CreateWidget` "/Game/UserInterface/Widgets/WB_TeamDisplayButton.WB_TeamDisplayButton_C" null _array_index))
              (`/Game/UserInterface/Widgets/WB_TeamDisplay.AddChildWidgetToGrid` (`self.ElestralsTeamDisplayRef`) _returnvalue_2)
              (`/Game/UserInterface/Widgets/WB_TeamDisplayButton.InitializeElestralVars` _returnvalue_2 _array_element))
            (`UserWidget.PlayAnimation` _elestralsteamdisplayref (`/Game/UserInterface/Widgets/WB_TeamDisplay.TeamAppear` _elestralsteamdisplayref) 0.0 1 "Forward" 1.0 false)
            (`WidgetBlueprintLibrary.SetInputMode_GameAndUIEx` self (`PanelWidget.GetChildAt` (`/Game/UserInterface/Widgets/WB_TeamDisplay.TeamList` (`self.ElestralsTeamDisplayRef`)) 0))
            (set `self.bShowMouseCursor` true)
            (bind (_direction _alpha) (`Timeline|LerpTime` :!via `PlayFromStart`)
              (:`Update`
                (`GameplayStatics.SetGlobalTimeDilation` (`KismetMathLibrary.Lerp` 0.1 1.0 _alpha)))
              (:`Finished`
                (`GameplayStatics.SetGamePaused` true)
                (`GameplayStatics.SetGlobalTimeDilation` 1.0)))))
        (:`B`
          (`WidgetBlueprintLibrary.SetInputMode_GameOnly` self :!label _label_2)
          (set `self.bShowMouseCursor` false)
          (`GameplayStatics.SetGamePaused` false)
          (if (`KismetSystemLibrary.IsValid` (`self.ElestralsTeamDisplayRef`))
            (`Widget.RemoveFromParent` (`self.ElestralsTeamDisplayRef`))
            (`TimelineComponent.Stop` (`self.LerpTime`))
            (`GameplayStatics.SetGlobalTimeDilation` 1.0)
            (if (`KismetSystemLibrary.IsValid` (`self.SummaryWidgetRef`))
              (`self.DisappearSummaryScreen`))
            (if (`KismetSystemLibrary.IsValid` (`self.SkillTreeWidgetRef`))
              (`Widget.RemoveFromParent` (`self.SkillTreeWidgetRef`)))
            (`KismetSystemLibrary.CollectGarbage`)))))))

(event `/Game/Blueprints/CentralClasses/BPI_UIUtils.RemoveTeamDisplayAtClashStart`
  ;[1 1 1] TeamDisplay Widget Appear and Initialize Logic
  (set `self.isInClash` true)
  (goto _label_2))

(event `EnhancedInput|/Game/ThirdPerson/Input/Actions/IA_DisplayCompendiumAction`
  (params (ActionValue :type Boolean) (ElapsedSeconds :type "Float (double-precision)") (TriggeredSeconds :type "Float (double-precision)") (InputAction :type "InputAction Object Reference" :default "/Game/ThirdPerson/Input/Actions/IA_DisplayCompendiumAction.IA_DisplayCompendiumAction"))
  (bind _playercharacterref (`self.PlayerCharacterRef`))
  ;[1 1 1] Create Compendium Actor
  (:`Started`
    (if (not (`self.isInClash`))
      (`/Engine/EditorBlueprintResources/StandardMacros.FlipFlop`
        (:`A`
          (set `self.isInCompendium` true)
          (bind _returnvalue (`|SpawnActorFromClass` "/Game/Blueprints/DiageticUI/BP_Compendium.BP_Compendium_C" (`KismetMathLibrary.MakeTransform` (+ (+ (* (`self.GetActorForwardVector` _playercharacterref) 80.0) (`self.K2_GetActorLocation` _playercharacterref)) (0.0 0.0 100.0)) (`KismetMathLibrary.MakeRotator` (.roll (`self.K2_GetActorRotation` _playercharacterref)) (.pitch (`self.K2_GetActorRotation` _playercharacterref)) (+ (.yaw (`self.K2_GetActorRotation` _playercharacterref)) 180.0))) "AlwaysSpawn" "MultiplyWithRoot" null (`AC_CompendiumBase.TotalElestralClassList` (`ElestralsCharacter.CompendiumComponent` _playercharacterref)) null))
          (bind _output_get (set `self.CompendiumRef` _returnvalue))
          (`self.Possess` _output_get))
        (:`B`
          (set `self.isInCompendium` false)
          (`self.Possess` (`self.PlayerCharacterRef`))
          (`self.K2_DestroyActor` (`self.CompendiumRef`)))))))

(event `self.ReceiveBeginPlay`
  ;[1 1 1] Initialize Pawn Refs
  (`|ExecutionSequence`
    (:`then_0`
      (bind _aselestrals_character (cast `ElestralsCharacter` (`GameplayStatics.GetPlayerPawn` 0)))
      (set `self.PlayerCharacterRef` _aselestrals_character)
      (set `self.Player Elestral Team Component` (`ElestralsCharacter.ElestralTeamComponent` (`self.PlayerCharacterRef`))))
    (:`then_1`
      (bind _returnvalue (`GameplayStatics.GetActorOfClass` "/Game/Materials/UI/BP_ElestralDisplay.BP_ElestralDisplay_C"))
      (set `self.Summary3DRef` _returnvalue))))

(event `/Game/Blueprints/CentralClasses/BPI_UIUtils.CreateSummaryWidget`
  (params (ElestralStatsStruct :type "ElestralStats Structure") (StatStructIndex :type Integer))
  ;[0.1296 1 0] Summary Widget Functionality
  (`self.CreateSummaryScreen` ElestralStatsStruct StatStructIndex))

(event `/Game/Blueprints/CentralClasses/BPI_UIUtils.CreateSkillTreeWidget`
  (params (StatStructIndex :type Integer))
  ;[0.2131 1 0] Skill Tree Functionality
  (bind _returnvalue (`|CreateWidget` "/Game/UserInterface/Widgets/WB_SkillTree.WB_SkillTree_C" null StatStructIndex (`|GetArrayItem` (`AC_ElestralsTeamComponent.TeamStatList` (`self.Player Elestral Team Component`)) StatStructIndex)))
  (bind _output_get (set `self.SkillTreeWidgetRef` _returnvalue))
  (`UserWidget.AddToViewport` _output_get 0)
  (`Widget.SetVisibility` (`self.SummaryWidgetRef`) "HitTestInvisible")
  (`UserWidget.PlayAnimation` _output_get (`/Game/UserInterface/Widgets/WB_SkillTree.Appear` _output_get) 0.0 1 "Forward" 1.0 false))

(event `/Game/Blueprints/CentralClasses/BPI_UIUtils.DestroySummaryWidget`
  ;[0.1296 1 0] Summary Widget Functionality
  (`self.DisappearSummaryScreen`))

(event `/Game/Blueprints/CentralClasses/BPI_UIUtils.UpdateStructWithMoveData`
  (params (StatStructIndex :type Integer) (SkillType :type "ESkillTypes Enum" :default "Light") (MoveData :type "ElestralsMoveBase Object Reference"))
  (bind _skilltreewidgetref (`self.SkillTreeWidgetRef`))
  (bind _output (`|GetArrayItem` (`AC_ElestralsTeamComponent.TeamStatList` (`self.Player Elestral Team Component`)) StatStructIndex))
  (bind _currentfollowingelestral (`AC_ElestralsTeamComponent.CurrentFollowingElestral` (`ElestralsCharacter.ElestralTeamComponent` (`self.PlayerCharacterRef`))))
  ;[0.2131 1 0] Skill Tree Functionality
  (`KismetSystemLibrary.PrintString` (`KismetStringLibrary.Conv_IntToString` StatStructIndex))
  (switch `ESkillTypes` SkillType
    (:`Light`
      (`KismetArrayLibrary.Array_Add` (`.CurrentActiveLightCombo` (break `ElestralStats` _output)) MoveData))
    (:`Heavy`
      (setmembers `ElestralStats` :`StructRef` _output :`CurrentActiveHeavyAttack` MoveData))
    (:`Ultimate`
      (setmembers `ElestralStats` :`StructRef` _output :`CurrentActiveUltimateAttack` MoveData)))
  (if (`KismetSystemLibrary.IsValid` _skilltreewidgetref)
    (message `/Game/Blueprints/CentralClasses/BPI_UIUtils.UpdateSkillTreeStruct` _skilltreewidgetref (`|GetArrayItem` (`AC_ElestralsTeamComponent.TeamStatList` (`self.Player Elestral Team Component`)) StatStructIndex))
    ;;[1 1 1] UPDATES ELESTRAL IF IT IS CURRENTLY FOLLOWING
    (if (`KismetSystemLibrary.IsValid` _currentfollowingelestral)
      (`self.UpdateStructValues` (cast `/Game/Blueprints/Elestrals/BP_ElestralBase` _currentfollowingelestral :!pure true)))))

(event `/Game/Blueprints/CentralClasses/BPI_UIUtils.SwapTeamDisplayToFront`
  (params (WidgetToSwap :type "/Game/UserInterface/Widgets/WB_TeamDisplayButton Object Reference"))
  (bind _teamlist (`/Game/UserInterface/Widgets/WB_TeamDisplay.TeamList` (`self.ElestralsTeamDisplayRef`)))
  ;[1 1 1] Team Display Button Swap Logic, maybe can refactor later to not create and destroy widgets but just swap data
  (set `self.tempChildIndex` (`PanelWidget.GetChildIndex` _teamlist WidgetToSwap))
  (for (_array_element _array_index) (`PanelWidget.GetAllChildren` _teamlist)
    (`Widget.RemoveFromParent` _array_element)
    (`KismetSystemLibrary.PrintString` (`KismetStringLibrary.Conv_IntToString` _array_index)))
  ;;[1 1 1] for some reason the above for each doesn't get rid of the last button so here's this
  (`Widget.RemoveFromParent` (`PanelWidget.GetChildAt` _teamlist 0))
  (`KismetSystemLibrary.CollectGarbage`)
  (if (not (== (`self.tempChildIndex`) 0))
    (`AC_ElestralsTeamComponent.SwapElestralTeamPositions` (`ElestralsCharacter.ElestralTeamComponent` (`self.PlayerCharacterRef`)) (`self.tempChildIndex`) 0))
  (`self.ReassessLoop`))

(event `EnhancedInput|/Game/ThirdPerson/Input/Actions/IA_Pause`
  (params (ActionValue :type Boolean) (ElapsedSeconds :type "Float (double-precision)") (TriggeredSeconds :type "Float (double-precision)") (InputAction :type "InputAction Object Reference" :default "/Game/ThirdPerson/Input/Actions/IA_Pause.IA_Pause"))
  ;[0.1399 1 0] Pause Functionality
  (:`Started`
    (if (`GameplayStatics.IsGamePaused`)
      (if (`KismetSystemLibrary.IsValid` (`self.PauseWidgetRef`)) :!label _label_3
        (`Widget.RemoveFromParent` (`self.PauseWidgetRef`))
        (`GameplayStatics.SetGamePaused` false))
      (else
        (bind _returnvalue (`|CreateWidget` "/Game/UserInterface/Settings/WB_Pause.WB_Pause_C"))
        (bind _output_get (set `self.PauseWidgetRef` _returnvalue))
        (`UserWidget.AddToViewport` _output_get 0)
        (`WidgetBlueprintLibrary.SetInputMode_GameAndUIEx` self (`/Game/UserInterface/Settings/WB_Pause.ResumeButton` (`self.PauseWidgetRef`)))
        (set `self.bShowMouseCursor` true)
        (`GameplayStatics.SetGamePaused` true)))))

(event `/Game/Blueprints/CentralClasses/BPI_UIUtils.UpdateStructValues`
  (params (PassedElestral :type "/Game/Blueprints/Elestrals/BP_ElestralBase Object Reference (by ref)"))
  (bind _output (`|GetArrayItem` (`AC_ElestralsTeamComponent.TeamStatList` (`self.Player Elestral Team Component`))))
  (bind ((`ElestralLevel` _elestrallevel) (`ElestralXPGrowthModifier` _elestralxpgrowthmodifier) (`CurrentActiveLightCombo` _currentactivelightcombo) (`CurrentActiveHeavyAttack` _currentactiveheavyattack) (`CurrentActiveUltimateAttack` _currentactiveultimateattack)) (break `ElestralStats` _output))
  ;[0.2131 1 0] Skill Tree Functionality
  (`AC_ElestralsData.SetElestralStats` (`CH_ElestralBase.ElestralDataComponent` PassedElestral) _output)
  (`KismetSystemLibrary.PrintString` (`KismetStringLibrary.Concat_StrStr` (`KismetStringLibrary.Conv_BoolToString` (`KismetArrayLibrary.Array_IsValidIndex` _currentactivelightcombo)) (`KismetStringLibrary.Conv_BoolToString` (`KismetSystemLibrary.IsValid` _currentactiveheavyattack)) (`KismetStringLibrary.Conv_BoolToString` (`KismetSystemLibrary.IsValid` _currentactiveultimateattack))) true true (struct :`R` 0.5934 :`G` 1.0 :`A` 1.0)))

(event `ReassessLoop`
  ;[1 1 1] Team Display Button Swap Logic, maybe can refactor later to not create and destroy widgets but just swap data
  (for (_array_element _array_index) (`AC_ElestralsTeamComponent.TeamStatList` (`self.Player Elestral Team Component`))
    (`self.ReassessTeamDisplay` _array_element _array_index))
  (`Widget.SetFocus` (`PanelWidget.GetChildAt` (`/Game/UserInterface/Widgets/WB_TeamDisplay.TeamList` (`self.ElestralsTeamDisplayRef`)) 0)))

(event `/Game/Blueprints/CentralClasses/BPI_UIUtils.ResumeFromPauseScreen`
  ;[0.1399 1 0] Pause Functionality
  (goto _label_3))

(event `/Game/Blueprints/CentralClasses/BPI_UIUtils.UpdateStructValuesFromElestral`
  (params (StatsToPass :type "ElestralStats Structure") (StatStructIndex :type Integer))
  (bind ((`ElestralLevel` _elestrallevel) (`ElestralXPGrowthModifier` _elestralxpgrowthmodifier) (`CurrentActiveLightCombo` _currentactivelightcombo) (`CurrentActiveHeavyAttack` _currentactiveheavyattack) (`CurrentActiveUltimateAttack` _currentactiveultimateattack) (`AllInstantiatedMoves` _allinstantiatedmoves)) (break `ElestralStats` StatsToPass))
  ;[0.2131 1 0] Skill Tree Functionality
  (setmembers `ElestralStats` :`StructRef` (`|GetArrayItem` (`AC_ElestralsTeamComponent.TeamStatList` (`self.Player Elestral Team Component`)) StatStructIndex) :`CurrentActiveLightCombo` _currentactivelightcombo :`CurrentActiveHeavyAttack` _currentactiveheavyattack :`CurrentActiveUltimateAttack` _currentactiveultimateattack :`AllInstantiatedMoves` _allinstantiatedmoves))

(event `/Game/Blueprints/CentralClasses/BPI_UIUtils.CreateSettingsWidget`
  ;[0.2631 1 0] Settings Functionality
  (bind _returnvalue (`|CreateWidget` "/Game/UserInterface/Settings/WB_Settings.WB_Settings_C"))
  (bind _output_get (set `self.SettingsWidgetRef` _returnvalue))
  (`UserWidget.AddToViewport` _output_get 0)
  (`Widget.SetVisibility` (`self.PauseWidgetRef`) "Hidden")
  (`Widget.SetFocus` (`/Game/UserInterface/Settings/WB_Settings.CloseSettingsButton` _output_get)))

(event `/Game/Blueprints/CentralClasses/BPI_UIUtils.CreateDialogueBox`
  (params (DialogueText :type Text))
  ;[0.1145 1 0] Dialogue Box Functionality
  (if (`KismetSystemLibrary.IsValid` (`self.currentDialogueBox`))
    (`KismetSystemLibrary.PrintString` "dialogue already on screen, can't create more")
    (else
      (bind _returnvalue (`|CreateWidget` "/Game/UserInterface/Widgets/WB_DialogueBox.WB_DialogueBox_C" null DialogueText))
      (bind _output_get (set `self.currentDialogueBox` _returnvalue))
      (`UserWidget.AddToViewport` _output_get 0)
      (bind _dialoguetextbutton (`/Game/UserInterface/Widgets/WB_DialogueBox.DialogueTextButton` _output_get))
      (`WidgetBlueprintLibrary.SetInputMode_GameAndUIEx` self _dialoguetextbutton)
      (`Widget.SetFocus` _dialoguetextbutton))))

(event `/Game/Blueprints/CentralClasses/BPI_UIUtils.DestroySkillTree`
  (params (`Team Stat Struct Index` :type Integer))
  ;[0.2131 1 0] Skill Tree Functionality
  (`self.DestroySkillTreeWidget` `Team Stat Struct Index`))

(event `/Game/Blueprints/CentralClasses/BPI_UIUtils.CloseSettingsWidget`
  (bind _pausewidgetref (`self.PauseWidgetRef`))
  ;[0.2631 1 0] Settings Functionality
  (`Widget.RemoveFromParent` (`self.SettingsWidgetRef`))
  (`Widget.SetVisibility` _pausewidgetref "SelfHitTestInvisible")
  (`Widget.SetFocus` (`/Game/UserInterface/Settings/WB_Pause.ResumeButton` _pausewidgetref)))

(event `/Game/Blueprints/CentralClasses/BPI_UIUtils.DestroyDialogueBox`
  (bind _currentdialoguebox (`self.currentDialogueBox`))
  ;[0.1145 1 0] Dialogue Box Functionality
  (if (`KismetSystemLibrary.IsValid` _currentdialoguebox)
    (`Widget.RemoveFromParent` _currentdialoguebox)
    (set `self.bShowMouseCursor` false)
    (`WidgetBlueprintLibrary.SetInputMode_GameOnly` self)
    (set `self.currentDialogueBox` null)))

(event `/Game/Blueprints/CentralClasses/BPI_UIUtils.UpdateIsInputtingCombo`
  (params (isInputtingCombo :type Boolean))
  ;[0.2131 1 0] Skill Tree Functionality
  (set `self.isInputtingCombo` isInputtingCombo))

(event `/Game/Blueprints/CentralClasses/BPI_UIUtils.ClearDataStructLightCombo`
  (params (StatStructIndex :type Integer))
  (bind ((`ElestralLevel` _elestrallevel) (`ElestralXPGrowthModifier` _elestralxpgrowthmodifier) (`CurrentActiveLightCombo` _currentactivelightcombo)) (break `ElestralStats` (`|GetArrayItem` (`AC_ElestralsTeamComponent.TeamStatList` (`self.Player Elestral Team Component`)) StatStructIndex)))
  ;[0.2131 1 0] Skill Tree Functionality
  (if (`KismetArrayLibrary.Array_IsValidIndex` _currentactivelightcombo)
    (`KismetArrayLibrary.Array_Clear` _currentactivelightcombo)))

(event `/Game/Blueprints/CentralClasses/BPI_ClashUtils.AddClashWidgetToScreen`
  (`self.CreateClashWidget`))

(event `/Game/Blueprints/CentralClasses/BPI_UIUtils.UpdatePlayerElestralHealthMeter`
  (params (HealthPercentage :type "Float (double-precision)"))
  (`self.UpdateHealthMeter` HealthPercentage))

(event `/Game/Blueprints/CentralClasses/BPI_UIUtils.UpdatePlayerElestralBondMeter`
  (params (BondPercentage :type "Float (double-precision)"))
  (`self.UpdateUltiMeter` BondPercentage))

(event `/Game/Blueprints/CentralClasses/BPI_ClashUtils.EndClash`
  (params (`Player Won?` :type Boolean))
  (set `self.isInClash` false)
  (`self.DestroyClashWidget`))

(fn `CreateClashWidget`
  (bind _returnvalue (`|CreateWidget` "/Game/UserInterface/Clash/WB_ClashMain.WB_ClashMain_C"))
  (bind _output_get (set `self.ClashWidgetRef` _returnvalue))
  (`UserWidget.AddToViewport` _output_get 0)
  (`/Game/UserInterface/Clash/WB_ClashMain.InitializeClashWidgetVarsForPlayer` _output_get (`AC_ElestralsData.ElestralStats` (`CH_ElestralBase.ElestralDataComponent` (`AC_ElestralsTeamComponent.CurrentFollowingElestral` (`ElestralsCharacter.ElestralTeamComponent` (`self.PlayerCharacterRef`)))))))

(fn `CreateSummaryScreen`
  (params (StatsToDisplay :type "ElestralStats Structure") (StatStructIndex :type Integer))
  (bind _summarywidgetref (`self.SummaryWidgetRef`))
  (`/Game/Materials/UI/BP_ElestralDisplay.SpawnSummaryElestral` (`self.Summary3DRef`) (`.ElestralClass` (break `ElestralStats` StatsToDisplay)))
  (bind _returnvalue (`AC_ElestralsData.SetElestralStats` (`CH_ElestralBase.ElestralDataComponent` (`/Game/Materials/UI/BP_ElestralDisplay.SpawnedElestral` (`self.Summary3DRef`))) (`|GetArrayItem` (`AC_ElestralsTeamComponent.TeamStatList` (`ElestralsCharacter.ElestralTeamComponent` (`self.PlayerCharacterRef`))) StatStructIndex)))
  (bind _returnvalue_2 (`|CreateWidget` "/Game/UserInterface/Widgets/WB_ElestralSummary.WB_ElestralSummary_C" null _returnvalue StatStructIndex))
  (bind _output_get (set `self.SummaryWidgetRef` _returnvalue_2))
  (`UserWidget.AddToViewport` _output_get 0)
  (`/Game/UserInterface/Widgets/WB_ElestralSummary.InitializeStatDisplay` _summarywidgetref)
  (set `UserWidget.bIsFocusable` true _summarywidgetref)
  (`UserWidget.PlayAnimation` _summarywidgetref (`/Game/UserInterface/Widgets/WB_ElestralSummary.AppearLeft` _returnvalue_2) 0.0 1 "Forward" 1.0 false)
  (`Widget.SetVisibility` (`self.ElestralsTeamDisplayRef`) "HitTestInvisible")
  (`Widget.SetFocus` (`/Game/UserInterface/Widgets/WB_ElestralSummary.SkillTreeButton` (`self.SummaryWidgetRef`))))

(fn `DestroyClashWidget`
  (`Widget.RemoveFromParent` (`self.ClashWidgetRef`)))

(fn `DestroySkillTreeWidget`
  (params (ElestralIndex :type Integer))
  (bind _summarywidgetref (`self.SummaryWidgetRef`))
  (bind _summarywidgetref_2 (`self.SummaryWidgetRef`))
  (`Widget.RemoveFromParent` (`self.SkillTreeWidgetRef`))
  (`Widget.SetVisibility` _summarywidgetref "SelfHitTestInvisible")
  (`Widget.SetFocus` (`/Game/UserInterface/Widgets/WB_ElestralSummary.SkillTreeButton` _summarywidgetref))
  ;[1 1 1] update summary widget after changing moves
  (if (`KismetSystemLibrary.IsValid` _summarywidgetref_2)
    (`AC_ElestralsData.SetElestralStats` (`CH_ElestralBase.ElestralDataComponent` (`/Game/Materials/UI/BP_ElestralDisplay.SpawnedElestral` (`self.Summary3DRef`))) (`|GetArrayItem` (`AC_ElestralsTeamComponent.TeamStatList` (`self.Player Elestral Team Component`)) ElestralIndex))
    (`/Game/UserInterface/Widgets/WB_ElestralSummary.InitializeStatDisplay` _summarywidgetref_2)))

(fn `DisappearSummaryScreen`
  (bind _elestralsteamdisplayref (`self.ElestralsTeamDisplayRef`))
  (`/Game/Materials/UI/BP_ElestralDisplay.ClearRender` (`self.Summary3DRef`))
  (`Widget.RemoveFromParent` (`self.SummaryWidgetRef`))
  (if (`KismetSystemLibrary.IsValid` _elestralsteamdisplayref)
    (`Widget.SetVisibility` _elestralsteamdisplayref "SelfHitTestInvisible")
    (`Widget.SetFocus` (`PanelWidget.GetChildAt` (`/Game/UserInterface/Widgets/WB_TeamDisplay.TeamList` _elestralsteamdisplayref) 0))))

(fn `NexusPlayerElestral`
  (params (IndexToChange :type Integer) (`Stat Struct` :type "ElestralStats Structure"))
  (`|VariableSetRef` (`|GetArrayItem` (`AC_ElestralsTeamComponent.TeamStatList` (`self.Player Elestral Team Component`)) IndexToChange) `Stat Struct`))

(fn `PossessFollowingElestral`
  (locals (CameraBlendTime :type "Float (single-precision)" :default 0.5))
  (bind _asbp_c_elestrals_player_character (cast `/Game/Blueprints/CentralClasses/BP_C_ElestralsPlayerCharacter` (`GameplayStatics.GetPlayerCharacter` 0)))
  (`self.SetViewTargetWithBlend` (`AC_ElestralsTeamComponent.CurrentFollowingElestral` (`ElestralsCharacter.ElestralTeamComponent` _asbp_c_elestrals_player_character)) (`local.CameraBlendTime`))
  (set `self.isInClash` true)
  (return))

(fn `ReassessTeamDisplay`
  (params (tempStats :type "ElestralStats Structure") (tempIndex :type Integer))
  (locals (indexTemp :type Integer))
  (bind _elestralsteamdisplayref (`self.ElestralsTeamDisplayRef`))
  (bind _aswb_team_display_button (cast `/Game/UserInterface/Widgets/WB_TeamDisplayButton` (`PanelWidget.GetChildAt` (`/Game/UserInterface/Widgets/WB_TeamDisplay.TeamList` _elestralsteamdisplayref) (`local.indexTemp`)) :!pure true))
  (bind _output_get (set `local.indexTemp` tempIndex))
  (bind _returnvalue (`|CreateWidget` "/Game/UserInterface/Widgets/WB_TeamDisplayButton.WB_TeamDisplayButton_C" null _output_get))
  (`/Game/UserInterface/Widgets/WB_TeamDisplay.AddChildWidgetToGrid` _elestralsteamdisplayref _returnvalue)
  (`/Game/UserInterface/Widgets/WB_TeamDisplayButton.InitializeElestralVars` _aswb_team_display_button tempStats)
  (`KismetSystemLibrary.PrintString` (`KismetStringLibrary.Conv_ObjectToString` _aswb_team_display_button) true true (struct :`R` 0.288738 :`B` 1.0 :`A` 1.0))
  (return))

(fn `SwapTeamDisplayChildren`
  (params (InChildIndex :type Integer))
  (locals (SwappingChildInitIndex :type Integer) (WasFirst :type "Widget Object Reference") (IsSwapping :type "Widget Object Reference")))

(fn `UpdateHealthMeter`
  (params (HealthPercentage :type "Float (double-precision)"))
  (bind _clashwidgetref (`self.ClashWidgetRef`))
  (if (`KismetSystemLibrary.IsValid` _clashwidgetref)
    (`ProgressBar.SetPercent` (`/Game/UserInterface/Clash/WB_ClashMain.HealthBar` _clashwidgetref) HealthPercentage)))

(fn `UpdateUltiMeter`
  (params (BondPercentage :type "Float (double-precision)"))
  (bind _clashwidgetref (`self.ClashWidgetRef`))
  (if (`KismetSystemLibrary.IsValid` _clashwidgetref)
    (`ProgressBar.SetPercent` (`/Game/UserInterface/Clash/WB_ClashMain.UltimateBar` _clashwidgetref) BondPercentage)))

(fn `UserConstructionScript`)