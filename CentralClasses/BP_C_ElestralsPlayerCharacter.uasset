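; Player character Blueprint for an Elestrals creature game, handling world interaction and the player's Elestral team.
; TryInteract spawns a trigger box ahead of the player through InteractionComponent to start dialogue.
; BeginPlay adds a starter Astrabbit to ElestralTeamComponent, spawns it as a follower, calculates its stats and writes them back to the team's first slot.
; Debug keys add clone members or destroy the follower; leftover test chains never run.
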(event EventBeginPlay
  (bind _elestralteamcomponent (Variables|Default|GetElestralTeamComponent))
  (|CallParentFunction)
  (bind _returnvalue (Class|ACElestralsTeamComponent|AddElestralStatstoTeam (Variables|Default|GetElestralTeamComponent) (Utilities|Struct|MakeElestralStats "OG ASTRABBIT" "Thunder" "Lunar" 1e+01 1.0 "/Game/Blueprints/Elestrals/BP_C_Astrabbit.BP_C_Astrabbit_C" "/Game/Art/ElestralModels/Astrabbit/Astrabbit_eyes_Bake1_PBR_Diffuse.Astrabbit_eyes_Bake1_PBR_Diffuse")))
  (Development|PrintString (Utilities|String|ToString(Float) (.elestralspeed _returnvalue)))
  (bind _returnvalue_2 (Class|ACElestralsTeamComponent|CreateFollowingElestral (Variables|Default|GetElestralTeamComponent)))
  (Variables|/Game/Blueprints/Elestrals/BP_ElestralBase.BP_ElestralBase_C|SetTeamComponentSpawnedFrom (.AsBP%20Elestral%20Base (Utilities|Casting|CastToBP_ElestralBase _returnvalue_2)) _elestralteamcomponent)
  (Class|ACElestralsData|CalculateElestralStats (Variables|/Script/Elestrals.CH_ElestralBase|GetElestralDataComponent (.AsBP%20Elestral%20Base (Utilities|Casting|CastToBP_ElestralBase _returnvalue_2))))
  (|SetBy-RefVar (Utilities|Array|Get(acopy) (Variables|/Script/Elestrals.AC_ElestralsTeamComponent|GetTeamStatList _elestralteamcomponent)) (Variables|/Script/Elestrals.AC_ElestralsData|GetElestralStats (Variables|/Script/Elestrals.CH_ElestralBase|GetElestralDataComponent (.AsBP%20Elestral%20Base (Utilities|Casting|CastToBP_ElestralBase _returnvalue_2)))))
  (Class|CHElestralBase|RefreshStructDataImplementation _returnvalue_2))

(event EventTryInteract
  (params (Value :type Input%20Action%20Value%20Structure%20%28by%20ref%29))
  (bind _returnvalue (Transformation|GetActorLocation))
  (bind _returnvalue_2 (Class|ACInteractionComponent|CreateInteractionTrigger (Variables|Default|GetInteractionComponent) "200.000000,200.000000,200.000000" _returnvalue (+ _returnvalue (* (Transformation|GetActorForwardVector) 5e+02)) (Math|Conversions|ToQuaternion(Rotator) (Transformation|GetActorRotation))))
  (if (Utilities|IsValid _returnvalue_2)
    (Class|BPIUIUtils|TryCreateDialogue(Message) _returnvalue_2)))

(event Input|KeyboardEvents|DebugKeyU
  (params (Key :type Key%20Structure :default "None") (ActionValue :type Input%20Action%20Value%20Structure)))

(event Input|KeyboardEvents|F
  (params (Key :type Key%20Structure :default "None"))
  (:Pressed
    (Class|ACElestralsTeamComponent|DestroyFollowingElestral (Variables|Default|GetElestralTeamComponent))))

(event Input|KeyboardEvents|Q
  (params (Key :type Key%20Structure :default "None"))
  ;[1 1 1] get from team ui screen elestral struct and then get specific struct from array
)

(event Input|KeyboardEvents|5
  (params (Key :type Key%20Structure :default "None"))
  (bind _tempdebughp (Variables|Default|Gettempdebughp))
  (:Pressed
    (Math|Float|IncrementFloat _tempdebughp
      (:%20%20
        (bind _returnvalue (Class|ACElestralsTeamComponent|AddElestralStatstoTeam (Variables|Default|GetElestralTeamComponent) (Utilities|Struct|MakeElestralStats "Astrabbit CLONEs" "Earth" "Earth" _tempdebughp 5e+01 1e+03 1e+01 2e+01 0.0 0.0 0.0 0.0 0.0 0.0 "/Game/Blueprints/Elestrals/BP_C_Astrabbit.BP_C_Astrabbit_C" "/Engine/EngineResources/AICON-Green.AICON-Green" 0 0 0 0)))
        (Development|PrintString (Utilities|String|ToString(Float) (.elestralspeed _returnvalue)))))))

(fn ConstructionScript
  (|CallParentFunction))