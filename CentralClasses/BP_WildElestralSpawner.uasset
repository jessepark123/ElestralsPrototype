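; Trigger volume that spawns a random wild Elestral when the player enters and starts a wild clash against the player's following Elestral.
; Each overlap spawns an AI pawn at a random point in the box, rolls its level within the min/max range, recalculates stats and runs wild init.
; The stats' class comes from a second random pick, so it can differ from the spawned pawn's class.
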(event `self.ReceiveActorBeginOverlap`
  (params (OtherActor :type "Actor Object Reference"))
  (bind _asbp_c_elestrals_player_character (cast `/Game/Blueprints/CentralClasses/BP_C_ElestralsPlayerCharacter` (`GameplayStatics.GetPlayerCharacter` 0) :!pure true))
  (cast `/Game/Blueprints/CentralClasses/BP_C_ElestralsPlayerCharacter` OtherActor)
  (bind _spawnedelestralref (`self.SpawnElestralInBox` (`KismetMathLibrary.RandomFloatInRange` (`KismetMathLibrary.Conv_IntToDouble` (`self.MinLevel`)) (`KismetMathLibrary.Conv_IntToDouble` (`self.MaxLevel`)))))
  (message `/Game/Blueprints/CentralClasses/BPI_ClashUtils.StartWildClash` (`GameplayStatics.GetGameState`) _spawnedelestralref (cast `/Game/Blueprints/Elestrals/BP_ElestralBase` (`AC_ElestralsTeamComponent.CurrentFollowingElestral` (`ElestralsCharacter.ElestralTeamComponent` _asbp_c_elestrals_player_character)) :!pure true) _asbp_c_elestrals_player_character))

(fn `SpawnElestralInBox`
  (params (`Elestral Level` :type "Float (single-precision)"))
  (returns (SpawnedElestralRef :type "/Game/Blueprints/Elestrals/BP_ElestralBase Object Reference"))
  (bind _outitem (`KismetArrayLibrary.Array_Random` (`self.ElestralsToSpawn`)))
  (bind _returnvalue (`AIBlueprintHelperLibrary.SpawnAIFromClass` _outitem "/Game/Blueprints/AI/ElestralsAI/BT_ElestralOverworld.BT_ElestralOverworld" (`KismetMathLibrary.RandomPointInBoundingBox` (`self.K2_GetActorLocation`) (`BoxComponent.GetScaledBoxExtent` (`self.SpawnerOverlap`))) (`KismetMathLibrary.MakeRotator` 0.0 0.0 (`KismetMathLibrary.RandomFloatInRange` 0.0 360.0)) false null))
  (bind _asbp_elestral_base (cast `/Game/Blueprints/Elestrals/BP_ElestralBase` _returnvalue))
  (bind _elestraldatacomponent (`CH_ElestralBase.ElestralDataComponent` _asbp_elestral_base))
  (bind _structout (setmembers `ElestralStats` :`StructRef` (`AC_ElestralsData.ElestralStats` _elestraldatacomponent) :`ElestralLevel` (`KismetMathLibrary.Conv_IntToDouble` (`KismetMathLibrary.FTrunc` `Elestral Level`)) :`ElestralClass` _outitem))
  (set `AC_ElestralsData.ElestralStats` _structout _elestraldatacomponent)
  (`AC_ElestralsData.CalculateElestralStats` _elestraldatacomponent)
  (set `/Game/Blueprints/Elestrals/BP_ElestralBase.isWildElestral` true _asbp_elestral_base)
  (`/Game/Blueprints/Elestrals/BP_ElestralBase.WildInit` _asbp_elestral_base)
  (return _asbp_elestral_base))

(fn `UserConstructionScript`)