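; Diegetic compendium actor for browsing Elestrals with move input.
; Vertical input lerps the view between top and bottom camera points via timelines, showing the star cone for the top view; horizontal input changes pages, with DoOnce gates throttling both.
; BeginPlay builds a duplicate-free class list from the total Elestral list.
; Each page briefly spawns that Elestral to read its stats struct, destroys it, then sets the name text.
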(event `MoveToTop`
  (bind _topcameraloc (`self.TopCameraLoc`))
  (bind _compendiumview (`self.CompendiumView`))
  (set `self.initCamLoc` (`SceneComponent.K2_GetComponentLocation` _compendiumview))
  (set `self.initCamRot` (`SceneComponent.K2_GetComponentRotation` _compendiumview))
  (`SceneComponent.SetHiddenInGame` (`self.StarCone`) false false)
  (bind (_direction _alpha) (`Timeline|LerpToTop` :!via `PlayFromStart`)
    (:`Update`
      (`SceneComponent.K2_SetWorldLocationAndRotation` (`self.CompendiumView`) (`KismetMathLibrary.VLerp` (`self.initCamLoc`) (`SceneComponent.K2_GetComponentLocation` _topcameraloc) _alpha) (`KismetMathLibrary.RLerp` (`self.initCamRot`) (`SceneComponent.K2_GetComponentRotation` _topcameraloc) _alpha true) false true))
    (:`Finished`
      (goto _label_2 :!via `Reset`))))

(event `MoveToBottom`
  (bind _compendiumview (`self.CompendiumView`))
  (bind _bottomcameraloc (`self.BottomCameraLoc`))
  (`self.InitializeCompendiumValueAtIndex` (`self.currentCompendiumIndex`))
  (set `self.initCamLoc` (`SceneComponent.K2_GetComponentLocation` _compendiumview))
  (set `self.initCamRot` (`SceneComponent.K2_GetComponentRotation` _compendiumview))
  (`SceneComponent.SetHiddenInGame` (`self.StarCone`) true false)
  (bind (_direction _alpha) (`Timeline|LerpToBottom` :!via `PlayFromStart`)
    (:`Update`
      (`SceneComponent.K2_SetWorldLocationAndRotation` (`self.CompendiumView`) (`KismetMathLibrary.VLerp` (`self.initCamLoc`) (`SceneComponent.K2_GetComponentLocation` _bottomcameraloc) _alpha) (`KismetMathLibrary.RLerp` (`self.initCamRot`) (`SceneComponent.K2_GetComponentRotation` _bottomcameraloc) _alpha true) false true))
    (:`Finished`
      (goto _label :!via `Reset`))))

(event `EnhancedInput|/Game/ThirdPerson/Input/Actions/IA_Move`
  (params (ActionValue :type "Vector2D Structure") (ElapsedSeconds :type "Float (double-precision)") (TriggeredSeconds :type "Float (double-precision)") (InputAction :type "InputAction Object Reference" :default "/Game/ThirdPerson/Input/Actions/IA_Move.IA_Move"))
  (:`Started`
    (`|ExecutionSequence`
      (:`then_0`
        (if (<= ActionValue_Y -0.9)
          (`/Engine/EditorBlueprintResources/StandardMacros.DoOnce` false :!label _label
            (:`Completed`
              (`self.MoveToTop`)))
          (elif (>= ActionValue_Y 0.9)
            (`/Engine/EditorBlueprintResources/StandardMacros.DoOnce` false :!label _label_2
              (:`Completed`
                (`self.MoveToBottom`))))))
      (:`then_1`
        (if (<= ActionValue_X -0.9)
          (`/Engine/EditorBlueprintResources/StandardMacros.DoOnce` false :!label _label_3
            (:`Completed`
              (`self.GoToPreviousCompendiumPage`)))
          (elif (>= ActionValue_X 0.9)
            (`/Engine/EditorBlueprintResources/StandardMacros.DoOnce` false :!label _label_4
              (:`Completed`
                (`self.GoToNextCompendiumPage`)))))))))

(event `GoToNextCompendiumPage`
  (if (`KismetSystemLibrary.IsValidClass` (`|GetArrayItem` (`self.FixedElestralList`) (+ (`self.currentCompendiumIndex`) 1)))
    (bind _result (`/Engine/EditorBlueprintResources/StandardMacros.IncrementInt` (`self.currentCompendiumIndex`))
      (:`  `
        (`self.InitializeCompendiumValueAtIndex` _result)
        (goto _label_3 :!via `Reset`)))))

(event `PopulateCompendiumDataRemoveDuplicates`
  (for _array_element (`self.TotalElestralList`)
    (bind _asbp_elestral_base (castclass `/Game/Blueprints/Elestrals/BP_ElestralBase` _array_element))
    (`KismetArrayLibrary.Array_AddUnique` (`self.FixedElestralList`) _asbp_elestral_base)
    (`KismetSystemLibrary.PrintString` (`KismetStringLibrary.Concat_StrStr` "added " (`KismetSystemLibrary.GetClassDisplayName` _asbp_elestral_base) " to compendium"))))

(event `GoToPreviousCompendiumPage`
  (if (`KismetSystemLibrary.IsValidClass` (`|GetArrayItem` (`self.FixedElestralList`) (- (`self.currentCompendiumIndex`) 1)))
    (bind _result (`/Engine/EditorBlueprintResources/StandardMacros.DecrementInt` (`self.currentCompendiumIndex`))
      (:`  `
        (`self.InitializeCompendiumValueAtIndex` _result)
        (goto _label_4 :!via `Reset`)))))

(event `self.ReceiveBeginPlay`
  (`self.PopulateCompendiumDataRemoveDuplicates`))

(event `InitializeCompendiumValueAtIndex`
  (params (CompendiumIndex :type Integer))
  (bind _returnvalue (`|SpawnActorFromClass` (`|GetArrayItem` (`self.FixedElestralList`) CompendiumIndex) (`KismetMathLibrary.MakeTransform` (0.0 0.0 0.0)) "AlwaysSpawn" "MultiplyWithRoot" null null))
  (bind _output_get (set `self.currentElestralStatStruct` (`AC_ElestralsData.ElestralStats` (`CH_ElestralBase.ElestralDataComponent` _returnvalue))))
  (`self.K2_DestroyActor` _returnvalue)
  (`TextRenderComponent.K2_SetText` (`self.ElestralNameText`) (`KismetSystemLibrary.MakeLiteralText` (`KismetTextLibrary.Conv_StringToText` (`.ElestralName` (break `ElestralStats` _output_get))))))

(fn `UserConstructionScript`)